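; GM_Gamemode is the game mode for a dice board game, setting up the pawn piece and die at start.
; BeginPlay reads player 0's cell from GI_GameInstance, converts it to a position through BoardRef, and spawns BP_Pion there and BP_Dice at the origin.
; RoleDiceAndMove only calls RollDice on the Dice reference, with no movement logic.
; Neither spawned actor is stored, and BoardRef and Dice are not assigned here.
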(event `self.ReceiveBeginPlay`
  (bind _asgi_game_instance (cast `/Game/Blueprint/GI_GameInstance` (`GameplayStatics.GetGameInstance`)))
  (`/Game/Blueprint/GI_GameInstance.GetPlayerCellByPlayerID` _asgi_game_instance 0)
  (bind _output_get (set `self.As GI Game Instance` _asgi_game_instance))
  (bind _playercellnumber (`/Game/Blueprint/GI_GameInstance.GetPlayerCellByPlayerID` _output_get 0))
  (bind _cell_position (`/Game/Blueprint/Board/BP_Board.Get Cell Position by Number` (`self.BoardRef`) _playercellnumber))
  (`|SpawnActorFromClass` "/Game/Blueprint/BP_Pion.BP_Pion_C" (`KismetMathLibrary.MakeTransform` _cell_position) "Undefined" "MultiplyWithRoot" null null)
  (`|SpawnActorFromClass` "/Game/Blueprint/BP_Dice.BP_Dice_C" (`KismetMathLibrary.MakeTransform` (0.0 0.0 0.0)) "Undefined" "MultiplyWithRoot" null null))

(fn `RoleDiceAndMove`
  (`/Game/Blueprint/BP_Dice.RollDice` (`self.Dice`)))

(fn `UserConstructionScript`)