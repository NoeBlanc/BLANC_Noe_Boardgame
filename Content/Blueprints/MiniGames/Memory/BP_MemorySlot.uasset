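; BP_MemorySlot is a clickable card slot for the Memory mini-game.
; On BeginPlay it registers in GM_Memory's SlotList, then after a short delay sets the cube's material from its Paire index.
; A click flips the slot after a delay by toggling root roll between 0 and 180 and inverting IsClickable, then notifies the game mode through OnSlotClicked.
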(event `self.ReceiveBeginPlay`
  ;[1 1 1] Set material ouaiiiis
  (bind _asgm_memory (cast `/Game/Blueprints/MiniGames/Memory/GM_Memory` (`GameplayStatics.GetGameMode`)))
  (bind _output_get (set `self.As GM Memory` _asgm_memory))
  (`KismetArrayLibrary.Array_AddUnique` (`/Game/Blueprints/MiniGames/Memory/GM_Memory.SlotList` _output_get) self)
  (`KismetSystemLibrary.Delay` 0.2)
  (switch `int` (`self.Paire`)
    (:`0`
      (`PrimitiveComponent.SetMaterial` (`self.Cube1`) 0 "/Game/Materials/MI_Action.MI_Action"))
    (:`1`
      (`PrimitiveComponent.SetMaterial` (`self.Cube1`) 0 "/Game/Materials/MI_BadAction.MI_BadAction"))
    (:`2`
      (`PrimitiveComponent.SetMaterial` (`self.Cube1`) 0 "/Game/LevelPrototyping/Materials/M_Solid.M_Solid"))
    (:`3`
      (`PrimitiveComponent.SetMaterial` (`self.Cube1`) 0 "/Game/Materials/MI_GoodAction.MI_GoodAction"))
    (:`4`
      (`PrimitiveComponent.SetMaterial` (`self.Cube1`) 0 "/Game/LevelPrototyping/Materials/MI_Solid_Blue.MI_Solid_Blue"))
    (:`5`
      (`PrimitiveComponent.SetMaterial` (`self.Cube1`) 0 "/Game/Materials/M_BaseMat.M_BaseMat"))))

(event `self.ReceiveActorOnClicked`
  (params (ButtonPressed :type "Key Structure"))
  (`KismetSystemLibrary.Delay` 0.3)
  (`self.ToggleSlot`)
  (`KismetSystemLibrary.Delay` 0.2)
  (`/Game/Blueprints/MiniGames/Memory/GM_Memory.OnSlotClicked` (`self.As GM Memory`) self))

(fn `ToggleSlot`
  (set `self.IsClickable` (not (`self.IsClickable`)))
  (if (== (.roll (.rotation (`SceneComponent.K2_GetComponentToWorld` (`self.DefaultSceneRoot`)))) 0.0)
    (`SceneComponent.K2_SetRelativeRotation` (`self.DefaultSceneRoot`) (`KismetMathLibrary.MakeRotator` 180.0) false false)
    (`KismetSystemLibrary.PrintString` "je retourne")
    (else
      (`SceneComponent.K2_SetRelativeRotation` :`self` (`self.DefaultSceneRoot`))
      (`KismetSystemLibrary.PrintString` "je suis caché mdr"))))

(fn `UserConstructionScript`)