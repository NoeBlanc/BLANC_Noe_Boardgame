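; BP_MemoryGamemaster sets up the pairs for a Memory minigame.
; On BeginPlay it gathers every BP_MemorySlot actor in the level into SlotList, then calls InitMemory.
; InitMemory shuffles the list and writes a pair ID to each slot, incrementing it after every second slot so neighbours in the shuffled order form random pairs.
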(event `self.ReceiveBeginPlay`
  (`|ExecutionSequence`
    (:`then_0`
      (bind _outactors (`GameplayStatics.GetAllActorsOfClass` "/Game/Blueprints/MiniGames/Memory/BP_MemorySlot.BP_MemorySlot_C"))
      (set `self.SlotList` _outactors))
    (:`then_1`
      (`self.InitMemory`))))

(fn `InitMemory`
  (locals (Int_paire :type Integer))
  (bind _slotlist (`self.SlotList`))
  (`KismetArrayLibrary.Array_Shuffle` _slotlist)
  (for (_array_element _array_index) _slotlist
    (set `/Game/Blueprints/MiniGames/Memory/BP_MemorySlot.Paire` (`local.Int_paire`) _array_element)
    (if (== (mod _array_index 2) 1)
      (`/Engine/EditorBlueprintResources/StandardMacros.IncrementInt` (`local.Int_paire`)))))

(fn `UserConstructionScript`)