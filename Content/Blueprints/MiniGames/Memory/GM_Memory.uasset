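; GM_Memory runs the card-matching memory minigame, judging slot clicks and detecting when the board is cleared.
; OnSlotClicked stores the first card as PreCard, then either destroys a matching pair and raises Score, or toggles both mismatched cards.
; Clicking the same card again clears the selection.
; When SlotList empties, CheckEnd increments the GameInstance's ScoreTemp, prints a points message and opens Test_map.
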(fn `CheckEnd`
  (if (== (`KismetArrayLibrary.Array_Length` (`self.SlotList`)) 0)
    (bind _result (`/Engine/EditorBlueprintResources/StandardMacros.IncrementInt` (`/Game/Blueprints/BP_GameInstance.ScoreTemp` (`self.GameInstanceRef`)))
      (:`  `
        (`KismetSystemLibrary.PrintString` (`KismetStringLibrary.Concat_StrStr` "You Gained" (`KismetStringLibrary.Conv_IntToString` _result) "Point"))
        (`GameplayStatics.OpenLevelBySoftObjectPtr` "/Game/Maps/Test_map.Test_map")))))

(fn `OnSlotClicked`
  (params (BP_SlotRef :type "/Game/Blueprints/MiniGames/Memory/BP_MemorySlot Object Reference"))
  (bind _precard (`self.PreCard`))
  (bind _precard_2 (`self.PreCard`))
  (bind _slotlist (`self.SlotList`))
  (if (`KismetSystemLibrary.IsValid` _precard)
    (if (== (`/Game/Blueprints/MiniGames/Memory/BP_MemorySlot.Paire` BP_SlotRef) (`/Game/Blueprints/MiniGames/Memory/BP_MemorySlot.Paire` _precard))
      (if (== BP_SlotRef _precard_2)
        (set `self.PreCard` null)
        (else
          (`/Engine/EditorBlueprintResources/StandardMacros.IncrementInt` (`self.Score`)
            (:`  `
              (`KismetArrayLibrary.Array_RemoveItem` _slotlist _precard_2)
              (`self.K2_DestroyActor` _precard_2)
              (`KismetArrayLibrary.Array_RemoveItem` _slotlist BP_SlotRef)
              (`self.K2_DestroyActor` BP_SlotRef)
              (set `self.PreCard` null)
              (`self.CheckEnd`)))))
      (else
        (`/Game/Blueprints/MiniGames/Memory/BP_MemorySlot.ToggleSlot` _precard_2)
        (`/Game/Blueprints/MiniGames/Memory/BP_MemorySlot.ToggleSlot` BP_SlotRef)
        (set `self.PreCard` null)))
    (else
      (set `self.PreCard` BP_SlotRef))))

(fn `UserConstructionScript`)