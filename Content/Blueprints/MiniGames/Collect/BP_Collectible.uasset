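; BP_Collectible is a pickup for the Collect minigame that adds its score to the game mode's total when overlapped.
; It caches GM_Collect on BeginPlay, and any overlap on its Collectible component raises GMScore without filtering the overlapping actor.
; A total of exactly five opens Test_map; otherwise it prints the score in French and destroys itself.
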(event `self.ReceiveBeginPlay`
  (bind _asgm_collect (cast `/Game/Blueprints/MiniGames/Collect/GM_Collect` (`GameplayStatics.GetGameMode`)))
  (set `self.As GM Collect` _asgm_collect))

(event `self.Collectible.OnComponentBeginOverlap`
  (params (OverlappedComponent :type "PrimitiveComponent Object Reference") (OtherActor :type "Actor Object Reference") (OtherComp :type "PrimitiveComponent Object Reference") (OtherBodyIndex :type Integer) (bFromSweep :type Boolean) (SweepResult :type "HitResult Structure (by ref)"))
  (bind _as_gm_collect (`self.As GM Collect`))
  (bind _output_get (set `/Game/Blueprints/MiniGames/Collect/GM_Collect.GMScore` (+ (`/Game/Blueprints/MiniGames/Collect/GM_Collect.GMScore` _as_gm_collect) (`CollectibleComponent.score` (`self.Collectible`))) _as_gm_collect))
  (if (== _output_get 5)
    (`GameplayStatics.OpenLevelBySoftObjectPtr` "/Game/Maps/Test_map.Test_map")
    (else
      (`KismetSystemLibrary.PrintString` (`KismetStringLibrary.Concat_StrStr` "Votre Score de collecte est : " (`KismetStringLibrary.Conv_IntToString` _output_get)))
      (`self.K2_DestroyActor`))))

(fn `UserConstructionScript`)