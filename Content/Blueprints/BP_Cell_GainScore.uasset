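; BP_Cell_GainScore is a cell Blueprint that awards one point to the player it acts on.
; Its Action override calls the parent, then reads that player's score by ID from BPGameInstance and writes it back incremented by one.
; A French debug Print String shows the player's ID and new total.
; All other graphs hold only default stubs or parent calls.
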(fn `Action`
  (params (PlayerID :type Integer) (PlayerStructure :type "Array of /Game/Blueprints/S_PlayerData Structure (by ref)"))
  (bind _as_bp_game_instance (`self.As BP Game Instance`))
  (`parent.Action` PlayerID PlayerStructure)
  (bind _playerscore (`/Game/Blueprints/BP_GameInstance.GetPlayerScoreByPlayerID` _as_bp_game_instance PlayerID))
  (bind _returnvalue (+ _playerscore 1))
  (`/Game/Blueprints/BP_GameInstance.SetPlayerScoreByPlayerID` _as_bp_game_instance PlayerID _returnvalue)
  (`KismetSystemLibrary.PrintString` (`KismetStringLibrary.Concat_StrStr` "Joueur" (`KismetStringLibrary.Conv_IntToString` PlayerID) "Possède" (`KismetStringLibrary.Conv_IntToString` _returnvalue)) true true (struct :`R` 1.0 :`B` 0.960651 :`A` 1.0)))

(fn `UserConstructionScript`
  (`parent.UserConstructionScript`))