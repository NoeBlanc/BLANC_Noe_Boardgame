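; Blueprint that simulates rolling a set of dice.
; RollDice rolls DiceNumber dice, each a random integer from 1 to DiceType, and sums them into ActualDiceResult.
; The total is shown on screen with a PrintString message, and the construction script is empty.
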(fn `RollDice`
  (set `self.ActualDiceResult` 0)
  (for _ (range 1 (+ (`self.DiceNumber`) 1))
    (bind _output_get (set `self.ActualDiceResult` (+ (`self.ActualDiceResult`) (`KismetMathLibrary.RandomIntegerInRange` 1 (`self.DiceType`))))))
  (`KismetSystemLibrary.PrintString` (`KismetStringLibrary.Concat_StrStr` "Your dice score is :" (`KismetStringLibrary.Conv_IntToString` _output_get))))

(fn `UserConstructionScript`)